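; BP_Gate is a two-leaf gate that opens when BP_FirstPersonCharacter overlaps its Box trigger.
; The overlap plays the DoorOpen timeline from the start, feeding its track to OpenGate for both pivots.
; OpenGate swings PivotLeft and PivotRight in opposite directions by lerping each current X direction vector toward an offset copy, re-read every update rather than from a stored start rotation.
; No closing logic exists.
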(event `self.Box.OnComponentBeginOverlap`
  (params (OverlappedComponent :type "PrimitiveComponent Object Reference") (OtherActor :type "Actor Object Reference") (OtherComp :type "PrimitiveComponent Object Reference") (OtherBodyIndex :type Integer) (bFromSweep :type Boolean) (SweepResult :type "HitResult Structure (by ref)"))
  (if (== (`GameplayStatics.GetObjectClass` OtherActor) "/Game/FirstPerson/Blueprints/BP_FirstPersonCharacter.BP_FirstPersonCharacter_C")
    (bind (_direction _doortrack) (`Timeline|DoorOpen` :!via `PlayFromStart`)
      (:`Update`
        (`self.OpenGate` _doortrack _doortrack)))))

(fn `OpenGate`
  (params (DoorTrack :type "Float (single-precision)") (DoorTrack2 :type "Float (single-precision)"))
  (bind _returnvalue (`KismetMathLibrary.Conv_RotatorToVector` (`SceneComponent.RelativeRotation` (`self.Pivot_Left`))))
  (bind _returnvalue_2 (`KismetMathLibrary.Conv_RotatorToVector` (`SceneComponent.RelativeRotation` (`self.Pivot_Right`))))
  (`SceneComponent.K2_SetRelativeRotation` (`self.Pivot_Left`) (`KismetMathLibrary.Conv_VectorToRotator` (`KismetMathLibrary.VLerp` _returnvalue (+ _returnvalue (0.0 -90.0 0.0)) DoorTrack)) false false)
  (`SceneComponent.K2_SetRelativeRotation` (`self.Pivot_Right`) (`KismetMathLibrary.Conv_VectorToRotator` (`KismetMathLibrary.VLerp` _returnvalue_2 (+ _returnvalue_2 (0.0 90.0 0.0)) DoorTrack2)) false false))

(fn `UserConstructionScript`)