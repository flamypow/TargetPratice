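; BP_Mallethazard is a swinging mallet hazard that knocks the first-person player character away on contact.
; A timeline started on BeginPlay lerps the actor's pitch between a starting and finishing angle, flipping playback direction each time it finishes to swing endlessly.
; Box overlap launches the character along the normalized vector from the actor's origin to the character, scaled by LaunchPower and added to its existing velocity.
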(event `self.ReceiveBeginPlay`
  (bind (_direction _swingtrack) (`Timeline|SwingTimeline`)
    (:`Update`
      (`self.K2_SetActorRotation` (`KismetMathLibrary.MakeRotator` 0.0 (`self.InterpAngle` _swingtrack))))
    (:`Finished`
      (`self.FlipDirections` _direction))))

(event `self.Box.OnComponentBeginOverlap`
  (params (OverlappedComponent :type "PrimitiveComponent Object Reference") (OtherActor :type "Actor Object Reference") (OtherComp :type "PrimitiveComponent Object Reference") (OtherBodyIndex :type Integer) (bFromSweep :type Boolean) (SweepResult :type "HitResult Structure (by ref)"))
  (bind _asbp_first_person_character (cast `/Game/FirstPerson/Blueprints/BP_FirstPersonCharacter` OtherActor))
  (`Character.LaunchCharacter` _asbp_first_person_character (* (`self.GetAwayDirection` _asbp_first_person_character) (`self.LaunchPower`)) false false))

(fn `FlipDirections`
  (params (A :type "ETimelineDirection Enum" :default "Forward"))
  (if (`|EnumEquality` A "Forward")
    (`TimelineComponent.Reverse` (`self.SwingTimeline`))
    (else
      (`TimelineComponent.Play` (`self.SwingTimeline`)))))

(fn `GetAwayDirection`
  (params (CharacterToLaunch :type "Actor Object Reference"))
  (returns (ReturnValue :type "Vector Structure"))
  (return (`KismetMathLibrary.Normal` (- (`self.K2_GetActorLocation` CharacterToLaunch) (`self.K2_GetActorLocation`)))))

(fn `InterpAngle`
  (params (Alpha :type "Float (double-precision)"))
  (returns (NewAngle :type "Float (double-precision)"))
  (return (`KismetMathLibrary.Lerp` (`self.StartingAngle`) (`self.FinishingAngle`) Alpha)))

(fn `UserConstructionScript`)